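; Player pawn Blueprint that sets up the local HUD and handles switching between a rifle and a launcher.
; On BeginPlay, the locally controlled pawn adds crosshair and health indicator widgets.
; ChangeWeapon input alternates through a FlipFlop between server events, launcher first, which swap both weapons between the active and unused mesh sockets and update CurrentWeapon.
; Radial damage only draws a debug sphere and prints the amount.
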(event `self.ReceiveBeginPlay`
  (if (`self.IsLocallyControlled`)
    (`|ExecutionSequence`
      (:`then_0`
        ;[1 1 1] Add Crosshair
        (bind _returnvalue (`|CreateWidget` "/Game/UI/WBP_Crosshair.WBP_Crosshair_C"))
        (`UserWidget.AddToViewport` _returnvalue 0))
      (:`then_1`
        ;[1 1 1] Add Health Indicator
        (bind _returnvalue_2 (`|CreateWidget` "/Game/UI/WBP_HealthIndicator.WBP_HealthIndicator_C"))
        (`UserWidget.AddToViewport` _returnvalue_2 0)))))

(event `ServerUseLauncher`
  ;[1 1 1] Change Weapon
  (`self.UseLauncher`))

(event `InputAction|ChangeWeapon`
  (params (Key :type "Key Structure"))
  ;[1 1 1] Change Weapon
  (:`Pressed`
    (`/Engine/EditorBlueprintResources/StandardMacros.FlipFlop`
      (:`A`
        (`self.ServerUseLauncher`))
      (:`B`
        (`self.ServerUseRifle`)))))

(event `ServerUseRifle`
  ;[1 1 1] Change Weapon
  (`self.UseRifle`))

(event `self.ReceiveRadialDamage`
  (params (DamageReceived :type "Float (single-precision)") (DamageType :type "DamageType Object Reference") (Origin :type "Vector Structure") (HitInfo :type "HitResult Structure (by ref)") (InstigatedBy :type "Controller Object Reference") (DamageCauser :type "Actor Object Reference"))
  (`KismetSystemLibrary.DrawDebugSphere` Origin 12.0 12 (struct :`R` 0.204661 :`G` 0.175239 :`B` 1.0 :`A` 1.0) 1.0 1.0)
  (`KismetSystemLibrary.PrintString` (`KismetStringLibrary.Concat_StrStr` "Player" ", dañado de rebote! " (`KismetStringLibrary.Conv_DoubleToString` DamageReceived))))

(fn `UseLauncher`
  (bind _secondweapon (`self.SecondWeapon`))
  (`self.K2_AttachToComponent` _secondweapon (`self.Mesh`) "WeaponSocket" "SnapToTarget" "SnapToTarget" "SnapToTarget" true)
  (`self.K2_AttachToComponent` (`self.PrimaryWeapon`) (`self.Mesh`) "UnusedWeaponSocket" "SnapToTarget" "SnapToTarget" "SnapToTarget" true)
  (set `self.CurrentWeapon` _secondweapon))

(fn `UserConstructionScript`)

(fn `UseRifle`
  (bind _primaryweapon (`self.PrimaryWeapon`))
  (`self.K2_AttachToComponent` _primaryweapon (`self.Mesh`) "WeaponSocket" "SnapToTarget" "SnapToTarget" "SnapToTarget" true)
  (`self.K2_AttachToComponent` (`self.SecondWeapon`) (`self.Mesh`) "UnusedWeaponSocket" "SnapToTarget" "SnapToTarget" "SnapToTarget" true)
  (set `self.CurrentWeapon` _primaryweapon))