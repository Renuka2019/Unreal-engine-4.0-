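; BP_TargetDummy is a target actor that gives debug feedback when it takes damage.
; Point damage draws a yellow debug sphere and the damage value at the hit location, and prints the damage with the dummy's name.
; Radial damage draws a larger red sphere at the damage origin and prints a splash-damage message.
; It tracks no health and only visualizes incoming damage.
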(event `self.ReceivePointDamage`
  (params (Damage :type "Float (single-precision)") (DamageType :type "DamageType Object Reference") (HitLocation :type "Vector Structure") (HitNormal :type "Vector Structure") (HitComponent :type "PrimitiveComponent Object Reference") (BoneName :type Name) (ShotFromDirection :type "Vector Structure") (InstigatedBy :type "Controller Object Reference") (DamageCauser :type "Actor Object Reference") (HitInfo :type "HitResult Structure (by ref)"))
  (`KismetSystemLibrary.DrawDebugSphere` HitLocation 5.0 12 (struct :`R` 1.0 :`G` 0.727552 :`B` 0.107261 :`A` 1.0) 1.0 1.0)
  (`KismetSystemLibrary.PrintString` (`KismetStringLibrary.Concat_StrStr` (`self.Name`) ", dañado! " " - " (`KismetStringLibrary.Conv_DoubleToString` Damage)))
  (`KismetSystemLibrary.DrawDebugString` HitLocation (`KismetStringLibrary.Conv_DoubleToString` Damage) null (struct :`R` 1.0 :`G` 1.0 :`B` 1.0 :`A` 1.0) 1.0))

(event `self.ReceiveRadialDamage`
  (params (DamageReceived :type "Float (single-precision)") (DamageType :type "DamageType Object Reference") (Origin :type "Vector Structure") (HitInfo :type "HitResult Structure (by ref)") (InstigatedBy :type "Controller Object Reference") (DamageCauser :type "Actor Object Reference"))
  (`KismetSystemLibrary.DrawDebugSphere` Origin 12.0 12 (struct :`R` 1.0 :`G` 0.24222 :`B` 0.16251 :`A` 1.0) 1.0 1.0)
  (`KismetSystemLibrary.PrintString` (`KismetStringLibrary.Concat_StrStr` (`self.Name`) ", dañado de rebote! " (`KismetStringLibrary.Conv_DoubleToString` DamageReceived))))

(fn `UserConstructionScript`)